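; Room actor that builds a dynamic mesh and its collision from a room's point outline, height and floor offset.
; Init runs the parent setup and then generates the mesh, and OnRebuildGeneratedMesh repeats that generation.
; Selection preview toggles wireframe, while Highlight shows polygroup colors until a retriggerable delay ends.
; The construction script fills the room data with a hardcoded five-point outline.
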(event `self.Init`
  (params (Room :type "DMRoom Structure"))
  (bind (_dmroom_height _dmroom_heightfromfloor _dmroom_points) (break `DMRoom` (`self.DMRoom`)))
  (bind _dynamicmeshcomponent (`self.DynamicMeshComponent`))
  (`parent.Init` Room)
  (bind _returnvalue (`BaseDynamicMeshComponent.GetDynamicMesh` _dynamicmeshcomponent :!label _label))
  (`/Game/Blueprints/Actors/Foundation/GeneratedActors_BP_Lib.Generate Spline Mesh` _returnvalue _dmroom_points _dmroom_height _dmroom_heightfromfloor)
  (`/Game/Blueprints/Actors/Foundation/GeneratedActors_BP_Lib.Generate Collision` _returnvalue _dynamicmeshcomponent))

(event `self.OnRebuildGeneratedMesh`
  (params (TargetMesh :type "DynamicMesh Object Reference"))
  (goto _label))

(event `self.ShowSelectionPreview`
  (set `BaseDynamicMeshComponent.bExplicitShowWireframe` true (`self.DynamicMeshComponent`)))

(event `self.HideSelectionPreview`
  (set `BaseDynamicMeshComponent.bExplicitShowWireframe` false (`self.DynamicMeshComponent`)))

(event `self.Highlight`
  (params (Duration :type "Float (single-precision)"))
  (bind _dynamicmeshcomponent (`self.DynamicMeshComponent`))
  (`BaseDynamicMeshComponent.SetColorOverrideMode` _dynamicmeshcomponent "Polygroups")
  (`BaseDynamicMeshComponent.SetColorOverrideMode` (`self.DynamicMeshComponent`) "Polygroups")
  (`KismetSystemLibrary.RetriggerableDelay` Duration)
  (`BaseDynamicMeshComponent.SetColorOverrideMode` _dynamicmeshcomponent "None"))

(fn `UserConstructionScript`
  (set `self.DMRoom` (make `DMRoom` 0.0 0.0 (`|MakeArray` (737.0 433.0) (540.0 435.0) (540.0 573.0) (714.0 553.0) (666.0 498.0) :!type "Vector2D Structure"))))