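; WallActor_BP is a wall actor that procedurally builds its dynamic mesh from wall, door and window data.
; On Init or mesh rebuild, it generates the wall from outline points, height and floor offset.
; Each door and window becomes a temporary mesh that is boolean-subtracted to cut openings, then collision is generated from the result.
; The construction script fills in a hardcoded sample wall and window.
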(event `self.Init`
  (params (Wall :type "DMWall Structure"))
  (bind (_dmwall_id _dmwall_name _dmwall_description _dmwall_enable _dmwall_visible _dmwall_area _dmwall_thickness _dmwall_connected _dmwall_thicknessavailability _dmwall_height _dmwall_heightfromfloor _dmwall_points) (break `DMWall` (`self.DMWall`)))
  (bind _dynamicmeshcomponent (`self.DynamicMeshComponent`))
  (`parent.Init` Wall)
  (bind _returnvalue (`BaseDynamicMeshComponent.GetDynamicMesh` _dynamicmeshcomponent :!label _label))
  (`/Game/Blueprints/Actors/Foundation/GeneratedActors_BP_Lib.Generate Spline Mesh` _returnvalue _dmwall_points _dmwall_height _dmwall_heightfromfloor)
  (`self.Generate Bool From Door Window Array` _returnvalue (`self.DMDoors`))
  (`self.Generate Bool From Door Window Array` _returnvalue (`self.DMWindows`))
  (`/Game/Blueprints/Actors/Foundation/GeneratedActors_BP_Lib.Generate Collision` _returnvalue _dynamicmeshcomponent))

(event `self.OnRebuildGeneratedMesh`
  (params (TargetMesh :type "DynamicMesh Object Reference"))
  (goto _label))

(fn `Generate Bool From Door Window Array`
  (params (Mesh :type "DynamicMesh Object Reference") (Array :type "Array of DMDoorWindow Structure"))
  (for _array_element Array
    (bind _returnvalue (`|GenericCreateObject` "/Script/GeometryFramework.DynamicMesh"))
    (`/Game/Blueprints/Actors/Foundation/GeneratedActors_BP_Lib.Generate Spline Mesh` _returnvalue (`.Points` (break `DMDoorWindow` _array_element)) (`.Height` (break `DMDoorWindow` _array_element)) (`.HeightFromFloor` (break `DMDoorWindow` _array_element)))
    (`GeometryScriptLibrary_MeshBooleanFunctions.ApplyMeshBoolean` Mesh (struct) _returnvalue (struct) "Subtract" (struct) null)))

(fn `UserConstructionScript`
  (set `self.DMWall` (make `DMWall` "" "" "" false false 0.0 0.0 false false 2.0 0.0 (`|MakeArray` (700.0 500.0) (710.0 500.0) (710.0 800.0) (700.0 800.0) (400.0 800.0) (400.0 790.0) (700.0 790.0) :!type "Vector2D Structure")))
  (`KismetArrayLibrary.Array_Add` (`self.DMWindows`) (make `DMDoorWindow` "" "" "" "" 0.0 false false 0.0 0.0 0.0 0.0 0.0 false 1.0 1.0 (`|MakeArray` (700.0 650.0) (710.0 650.0) (710.0 750.0) (700.0 750.0) :!type "Vector2D Structure"))))