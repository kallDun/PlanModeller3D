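; Generated wall actor that builds a procedural wall mesh with door and window openings using dynamic meshes.
; On init or rebuild, it generates a mesh from the wall's points, height and floor offset.
; Each door and window becomes a temporary mesh of the same kind, boolean-subtracted from the wall.
; The construction script fills the wall data with hardcoded sample values.
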(event `self.Init`
  (params (Wall :type "DMWall Structure"))
  (bind (_dmwall_id _dmwall_name _dmwall_description _dmwall_enable _dmwall_visible _dmwall_area _dmwall_thickness _dmwall_connected _dmwall_thicknessavailability _dmwall_height _dmwall_heightfromfloor _dmwall_points) (break `DMWall` (`self.DMWall`)))
  (`parent.Init` Wall)
  (bind _returnvalue (`BaseDynamicMeshComponent.GetDynamicMesh` (`self.DynamicMeshComponent`) :!label _label))
  (`/Game/Blueprints/Actors/Generated/GeneratedActors_BP_Lib.Generate Spline Mesh` _returnvalue _dmwall_points _dmwall_height _dmwall_heightfromfloor)
  (`self.Generate Bool From Door Window Array` _returnvalue (`self.DMDoors`))
  (`self.Generate Bool From Door Window Array` _returnvalue (`self.DMWindows`)))

(event `self.OnRebuildGeneratedMesh`
  (params (TargetMesh :type "DynamicMesh Object Reference"))
  (goto _label))

(fn `Generate Bool From Door Window Array`
  (params (Mesh :type "DynamicMesh Object Reference") (Array :type "Array of DMDoorWindow Structure"))
  (for _array_element Array
    (bind _returnvalue (`|GenericCreateObject` "/Script/GeometryFramework.DynamicMesh"))
    (`/Game/Blueprints/Actors/Generated/GeneratedActors_BP_Lib.Generate Spline Mesh` _returnvalue (`.Points` (break `DMDoorWindow` _array_element)) (`.Height` (break `DMDoorWindow` _array_element)) (`.HeightFromFloor` (break `DMDoorWindow` _array_element)))
    (`GeometryScriptLibrary_MeshBooleanFunctions.ApplyMeshBoolean` Mesh (struct) _returnvalue (struct) "Subtract" (struct) null)))

(fn `UserConstructionScript`
  (set `self.DMWall` (make `DMWall` "" "" "" false false 0.0 0.0 false false 2.0 0.0 (`|MakeArray` (714.2 553.1) (666.8 498.2) (672.5 493.4) (719.9 548.3) :!type "Vector2D Structure"))))