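; Chair furniture actor, a child Blueprint that builds on parent placement logic.
; The construction script registers its mesh in the inherited Meshes list, and the view visibility update sets that mesh visible.
; CheckPlacement returns the parent's result and swaps the mesh's material list between the normal chair materials and an all-red set to flag invalid placement.
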(fn `CheckPlacement`
  (returns (ReturnValue :type Boolean))
  (bind _furnituremesh (`self.FurnitureMesh`))
  (bind _returnvalue (`parent.CheckPlacement`))
  (`|ExecutionSequence`
    (:`then_0`
      (if _returnvalue
        (`GeometryScriptLibrary_SceneUtilityFunctions.SetComponentMaterialList` _furnituremesh (`|MakeArray` "/Game/ThirdParty/LoftOffice/Materials/M_Chair_3_plastic.M_Chair_3_plastic" "/Game/ThirdParty/LoftOffice/Materials/M_Chair_bottom.M_Chair_bottom" "/Game/ThirdParty/LoftOffice/Materials/M_Chair_seat.M_Chair_seat" "/Game/ThirdParty/LoftOffice/Materials/M_Chair_chrome.M_Chair_chrome" :!type "MaterialInterface Object Reference") null)
        (else
          (`GeometryScriptLibrary_SceneUtilityFunctions.SetComponentMaterialList` _furnituremesh (`|MakeArray` "/AnimationSharing/AnimSharingRed.AnimSharingRed" "/AnimationSharing/AnimSharingRed.AnimSharingRed" "/AnimationSharing/AnimSharingRed.AnimSharingRed" "/AnimationSharing/AnimSharingRed.AnimSharingRed" :!type "MaterialInterface Object Reference") null))))
    (:`then_1`
      (return _returnvalue))))

(fn `Update View Visibility`
  (params (`View Name` :type String))
  (switch `string` `View Name`
    (:`Default`
      (`SceneComponent.SetVisibility` (`self.FurnitureMesh`) true false))))

(fn `UserConstructionScript`
  (`parent.UserConstructionScript`)
  (`KismetArrayLibrary.Array_Add` (`self.Meshes`) (`self.FurnitureMesh`)))