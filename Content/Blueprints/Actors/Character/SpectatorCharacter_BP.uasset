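; SpectatorCharacter_BP is a free-camera spectator character that also relays player input to an active instrument.
; Enhanced Input moves it by a settings-driven speed with swept offsets, reversing the step on a blocking hit, and turns the camera through controller yaw and pitch.
; Property updates apply camera FOV and capsule collision from character settings.
; Instrument actions and Tick pass input structs to the valid ActiveInstrument, covering use, exit and axis values.
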(event `EnhancedInput|/Game/Blueprints/Actors/Character/Input/PlayerMovement_IA`
  (params (ActionValue :type "Vector2D Structure") (ElapsedSeconds :type "Float (double-precision)") (TriggeredSeconds :type "Float (double-precision)") (InputAction :type "InputAction Object Reference" :default "/Game/Blueprints/Actors/Character/Input/PlayerMovement_IA.PlayerMovement_IA"))
  (bind (_returnvalue_biscurrentcharacter _returnvalue_bwasplayedbefore _returnvalue_bresetlocationandrotation _returnvalue_savedlocation _returnvalue_savedrotation _returnvalue_camerafov _returnvalue_cameraspeed _returnvalue_biscolliding) (break `CharacterSettings` (`self.GetCharacterSettings`)))
  (bind _returnvalue (* ActionValue_Y _returnvalue_cameraspeed))
  (bind _returnvalue_2 (* ActionValue_X _returnvalue_cameraspeed))
  (:`Triggered`
    (bind _sweephitresult (`self.K2_AddActorLocalOffset` (`KismetMathLibrary.MakeVector` _returnvalue_2 _returnvalue) true))
    (if (`GameplayStatics.BreakHitResult` _sweephitresult)
      (`self.K2_AddActorLocalOffset` (`KismetMathLibrary.MakeVector` (* _returnvalue_2 -1.0) (* _returnvalue -1.0))))))

(event `EnhancedInput|/Game/Blueprints/Actors/Character/Input/CameraMovement_IA`
  (params (ActionValue :type "Vector2D Structure") (ElapsedSeconds :type "Float (double-precision)") (TriggeredSeconds :type "Float (double-precision)") (InputAction :type "InputAction Object Reference" :default "/Game/Blueprints/Actors/Character/Input/CameraMovement_IA.CameraMovement_IA"))
  (:`Triggered`
    (`self.AddControllerYawInput` ActionValue_X)
    (`self.AddControllerPitchInput` (* ActionValue_Y -1.0))))

(event `self.OnUpdateProperties`
  (bind (_returnvalue_biscurrentcharacter _returnvalue_bwasplayedbefore _returnvalue_bresetlocationandrotation _returnvalue_savedlocation _returnvalue_savedrotation _returnvalue_camerafov _returnvalue_cameraspeed _returnvalue_biscolliding) (break `CharacterSettings` (`self.GetCharacterSettings`)))
  (`CameraComponent.SetFieldOfView` (`self.Camera`) _returnvalue_camerafov)
  (`PrimitiveComponent.SetCollisionEnabled` (`self.CapsuleComponent`) (select `bool` _returnvalue_biscolliding :`false` "NoCollision" :`true` "QueryAndPhysics" :!type "ECollisionEnabled Enum")))

(event `self.ReceiveTick`
  (params (DeltaSeconds :type "Float (single-precision)"))
  (bind _activeinstrument (`self.ActiveInstrument`))
  (`/Engine/EditorBlueprintResources/StandardMacros.IsValid` _activeinstrument
    (:`Is Valid`
      (`CharacterInstrument.Input` _activeinstrument (make `InstrumentInputData` false false true)))))

(event `EnhancedInput|/Game/Blueprints/Actors/Character/Input/InstrumentUsing_IA`
  (params (ActionValue :type Boolean) (ElapsedSeconds :type "Float (double-precision)") (TriggeredSeconds :type "Float (double-precision)") (InputAction :type "InputAction Object Reference" :default "/Game/Blueprints/Actors/Character/Input/InstrumentUsing_IA.InstrumentUsing_IA"))
  (bind _activeinstrument (`self.ActiveInstrument`))
  (:`Triggered`
    (`/Engine/EditorBlueprintResources/StandardMacros.IsValid` _activeinstrument
      (:`Is Valid`
        (`CharacterInstrument.Input` _activeinstrument (make `InstrumentInputData` false true))))))

(event `EnhancedInput|/Game/Blueprints/Actors/Character/Input/InstrumentClosing_IA`
  (params (ActionValue :type Boolean) (ElapsedSeconds :type "Float (double-precision)") (TriggeredSeconds :type "Float (double-precision)") (InputAction :type "InputAction Object Reference" :default "/Game/Blueprints/Actors/Character/Input/InstrumentClosing_IA.InstrumentClosing_IA"))
  (bind _activeinstrument (`self.ActiveInstrument`))
  (:`Triggered`
    (`/Engine/EditorBlueprintResources/StandardMacros.IsValid` _activeinstrument
      (:`Is Valid`
        (`CharacterInstrument.Input` _activeinstrument (make `InstrumentInputData` true))))))

(event `EnhancedInput|/Game/Blueprints/Actors/Character/Input/InstrumentAxis2_IA`
  (params (ActionValue :type "Vector2D Structure") (ElapsedSeconds :type "Float (double-precision)") (TriggeredSeconds :type "Float (double-precision)") (InputAction :type "InputAction Object Reference" :default "/Game/Blueprints/Actors/Character/Input/InstrumentAxis2_IA.InstrumentAxis2_IA"))
  (bind _activeinstrument (`self.ActiveInstrument`))
  (:`Triggered`
    (`/Engine/EditorBlueprintResources/StandardMacros.IsValid` _activeinstrument
      (:`Is Valid`
        (`CharacterInstrument.Input` _activeinstrument (make `InstrumentInputData` false false false ActionValue))))))

(event `EnhancedInput|/Game/Blueprints/Actors/Character/Input/InstrumentAxis1_IA`
  (params (ActionValue :type "Float (double-precision)") (ElapsedSeconds :type "Float (double-precision)") (TriggeredSeconds :type "Float (double-precision)") (InputAction :type "InputAction Object Reference" :default "/Game/Blueprints/Actors/Character/Input/InstrumentAxis1_IA.InstrumentAxis1_IA"))
  (bind _activeinstrument (`self.ActiveInstrument`))
  (:`Triggered`
    (`/Engine/EditorBlueprintResources/StandardMacros.IsValid` _activeinstrument
      (:`Is Valid`
        (`CharacterInstrument.Input` _activeinstrument (make `InstrumentInputData` false false false (struct) ActionValue))))))

(event `EnhancedInput|/Game/Blueprints/Actors/Character/Input/InstrumentTriggerNext_IA`
  (params (ActionValue :type Boolean) (ElapsedSeconds :type "Float (double-precision)") (TriggeredSeconds :type "Float (double-precision)") (InputAction :type "InputAction Object Reference" :default "/Game/Blueprints/Actors/Character/Input/InstrumentTriggerNext_IA.InstrumentTriggerNext_IA"))
  (bind _activeinstrument (`self.ActiveInstrument`))
  (:`Triggered`
    (`/Engine/EditorBlueprintResources/StandardMacros.IsValid` _activeinstrument
      (:`Is Valid`
        (`CharacterInstrument.Input` _activeinstrument (make `InstrumentInputData` false false false (struct) 0.0 true))))))

(event `EnhancedInput|/Game/Blueprints/Actors/Character/Input/InstrumentTriggerPrevious_IA`
  (params (ActionValue :type Boolean) (ElapsedSeconds :type "Float (double-precision)") (TriggeredSeconds :type "Float (double-precision)") (InputAction :type "InputAction Object Reference" :default "/Game/Blueprints/Actors/Character/Input/InstrumentTriggerPrevious_IA.InstrumentTriggerPrevious_IA"))
  (bind _activeinstrument (`self.ActiveInstrument`))
  (:`Triggered`
    (`/Engine/EditorBlueprintResources/StandardMacros.IsValid` _activeinstrument
      (:`Is Valid`
        (`CharacterInstrument.Input` _activeinstrument (make `InstrumentInputData` false false false (struct) 0.0 false true))))))

(event `EnhancedInput|/Game/Blueprints/Actors/Character/Input/InstrumentUndo_IA`
  (params (ActionValue :type Boolean) (ElapsedSeconds :type "Float (double-precision)") (TriggeredSeconds :type "Float (double-precision)") (InputAction :type "InputAction Object Reference" :default "/Game/Blueprints/Actors/Character/Input/InstrumentUndo_IA.InstrumentUndo_IA"))
  (bind _activeinstrument (`self.ActiveInstrument`))
  (:`Triggered`
    (`/Engine/EditorBlueprintResources/StandardMacros.IsValid` _activeinstrument
      (:`Is Valid`
        (`CharacterInstrument.Input` _activeinstrument (make `InstrumentInputData` false false false (struct) 0.0 false false true))))))

(fn `UserConstructionScript`)