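; SpectatorCharacter_BP is a free-flying spectator pawn that moves the camera and drives the player's active instrument.
; Enhanced Input moves it by swept local X/Y offsets, applying an opposite offset on blocking hits, and rotates the controller for look.
; Character settings supply speed, FOV and whether the capsule collides.
; The active instrument previews every tick; input actions use it or deactivate it through the instruments manager.
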(event `EnhancedInput|/Game/Blueprints/Controllers/Character/Input/PlayerMovement_IA`
  (params (ActionValue :type "Vector2D Structure") (ElapsedSeconds :type "Float (double-precision)") (TriggeredSeconds :type "Float (double-precision)") (InputAction :type "InputAction Object Reference" :default "/Game/Blueprints/Controllers/Character/Input/PlayerMovement_IA.PlayerMovement_IA"))
  (bind (_returnvalue_biscurrentcharacter _returnvalue_bwasplayedbefore _returnvalue_bresetlocationandrotation _returnvalue_savedlocation _returnvalue_savedrotation _returnvalue_camerafov _returnvalue_cameraspeed _returnvalue_biscolliding) (break `CharacterSettings` (`self.GetCharacterSettings`)))
  (bind _returnvalue (* ActionValue_Y _returnvalue_cameraspeed))
  (bind _returnvalue_2 (* ActionValue_X _returnvalue_cameraspeed))
  (:`Triggered`
    (bind _sweephitresult (`self.K2_AddActorLocalOffset` (`KismetMathLibrary.MakeVector` _returnvalue_2 _returnvalue) true))
    (if (`GameplayStatics.BreakHitResult` _sweephitresult)
      (`self.K2_AddActorLocalOffset` (`KismetMathLibrary.MakeVector` (* _returnvalue_2 -1.0) (* _returnvalue -1.0))))))

(event `EnhancedInput|/Game/Blueprints/Controllers/Character/Input/CameraMovement_IA`
  (params (ActionValue :type "Vector2D Structure") (ElapsedSeconds :type "Float (double-precision)") (TriggeredSeconds :type "Float (double-precision)") (InputAction :type "InputAction Object Reference" :default "/Game/Blueprints/Controllers/Character/Input/CameraMovement_IA.CameraMovement_IA"))
  (:`Triggered`
    (`self.AddControllerYawInput` ActionValue_X)
    (`self.AddControllerPitchInput` (* ActionValue_Y -1.0))))

(event `self.OnUpdateProperties`
  (bind (_returnvalue_biscurrentcharacter _returnvalue_bwasplayedbefore _returnvalue_bresetlocationandrotation _returnvalue_savedlocation _returnvalue_savedrotation _returnvalue_camerafov _returnvalue_cameraspeed _returnvalue_biscolliding) (break `CharacterSettings` (`self.GetCharacterSettings`)))
  (`CameraComponent.SetFieldOfView` (`self.Camera`) _returnvalue_camerafov)
  (`PrimitiveComponent.SetCollisionEnabled` (`self.CapsuleComponent`) (select `bool` _returnvalue_biscolliding :`false` "NoCollision" :`true` "QueryAndPhysics" :!type "ECollisionEnabled Enum")))

(event `self.ReceiveTick`
  (params (DeltaSeconds :type "Float (single-precision)"))
  (bind _activeinstrument (`self.ActiveInstrument`))
  (`/Engine/EditorBlueprintResources/StandardMacros.IsValid` _activeinstrument
    (:`Is Valid`
      (`CharacterInstrument.Preview` _activeinstrument))))

(event `EnhancedInput|/Game/Blueprints/Controllers/Character/Input/InstrumentUsing_IA`
  (params (ActionValue :type Boolean) (ElapsedSeconds :type "Float (double-precision)") (TriggeredSeconds :type "Float (double-precision)") (InputAction :type "InputAction Object Reference" :default "/Game/Blueprints/Controllers/Character/Input/InstrumentUsing_IA.InstrumentUsing_IA"))
  (bind _activeinstrument (`self.ActiveInstrument`))
  (:`Triggered`
    (`/Engine/EditorBlueprintResources/StandardMacros.IsValid` _activeinstrument
      (:`Is Valid`
        (`CharacterInstrument.Use` _activeinstrument)))))

(event `EnhancedInput|/Game/Blueprints/Controllers/Character/Input/InstrumentClosing_IA`
  (params (ActionValue :type Boolean) (ElapsedSeconds :type "Float (double-precision)") (TriggeredSeconds :type "Float (double-precision)") (InputAction :type "InputAction Object Reference" :default "/Game/Blueprints/Controllers/Character/Input/InstrumentClosing_IA.InstrumentClosing_IA"))
  (:`Triggered`
    (`/Engine/EditorBlueprintResources/StandardMacros.IsValid` (`self.ActiveInstrument`)
      (:`Is Valid`
        (`InstrumentsManager.DeactivateCurrentInstrument` (`CoreFunctionLib.GetInstrumentsManager`))))))

(fn `UserConstructionScript`)